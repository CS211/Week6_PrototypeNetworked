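; Matchmaker Blueprint that automatically puts the first local player into an online multiplayer session on BeginPlay.
; It searches for non-LAN sessions and joins the first result.
; If the search returns none, it creates a session and opens the level named by LevelString as a listen server.
; Find, create and join failures are only printed, with no retry.
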(event EventBeginPlay
  (Development|PrintString "event begin play")
  (bind _results (|FindSessions (Game|GetPlayerController 0) 4 false)
    (:OnSuccess
      (if (== (Utilities|Array|Length _results) 0)
        (|Session (Game|GetPlayerController 0) 4 false
          (:OnSuccess
            (Game|OpenLevel(byName) (Variables|Default|GetLevelString) true "listen"))
          (:OnFailure
            (Development|PrintString "Create Session Fail")))
        (else
          (Development|PrintString (Utilities|String|ToString(Integer) (Utilities|Array|Length _results)))
          (|JoinSession (Game|GetPlayerController 0) (Utilities|Array|Get(acopy) _results)
            (:OnFailure
              (Development|PrintString "JoinSessionFailed"))))))
    (:OnFailure
      (Development|PrintString "Find Sessions Failed"))))

(event EventActorBeginOverlap
  (params (OtherActor :type Actor%20Object%20Reference)))

(event EventTick
  (params (DeltaSeconds :type Float%20%28single-precision%29)))

(fn ConstructionScript)